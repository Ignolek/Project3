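; Checkpoint actor that registers itself as the running character's last checkpoint when that character overlaps its box.
; Each overlap also stores the actor's location in Position.
; The first overlap unlocks it, plays a sound and shows CheckpointUI widgets for a few seconds before hiding them.
; Each checkpoint adds its own widget at BeginPlay, and the display toggle finds top-level widgets by class.
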(event OnComponentBeginOverlap(Box)
  (params (OverlappedComponent :type Primitive%20Component%20Object%20Reference) (OtherActor :type Actor%20Object%20Reference) (OtherComp :type Primitive%20Component%20Object%20Reference) (OtherBodyIndex :type Integer) (bFromSweep :type Boolean) (SweepResult :type Hit%20Result%20Structure%20%28by%20ref%29))
  (bind _asbp_running_character (Utilities|Casting|CastToBP_RunningCharacter OtherActor))
  (Variables|/Game/Blueprints/GameModeClasses/BP_RunningCharacter.BP_RunningCharacter_C|SetLastCheckpoint _asbp_running_character self)
  (Variables|Default|SetPosition (Transformation|GetActorLocation))
  (if (not (Variables|Default|Getunlocked))
    (Audio|PlaySound2D "/Game/SFX/lowRandom.lowRandom" 1.0 1.0 0.0 0 0)
    (Variables|Default|Setunlocked true)
    (bind _foundwidgets (Widget|GetAllWidgetsOfClass "/Game/UI/CheckpointUI.CheckpointUI_C" true))
    (Widget|SetVisibility _foundwidgets "Visible")
    (Utilities|FlowControl|Delay 3.0)
    (Widget|SetVisibility _foundwidgets "Hidden")))

(event EventBeginPlay
  (bind _returnvalue (UserInterface|CreateWidget "/Game/UI/CheckpointUI.CheckpointUI_C"))
  (UserInterface|Viewport|AddtoViewport _returnvalue 0))

(event Collision|EventActorBeginOverlap
  (params (OtherActor :type Actor%20Object%20Reference)))

(event EventTick
  (params (DeltaSeconds :type Float%20%28single-precision%29)))

(fn ConstructionScript)