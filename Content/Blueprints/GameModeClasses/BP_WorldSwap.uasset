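; BP_WorldSwap swaps between red and blue worlds while the left or right mouse button is held, making that color's platforms solid.
; Press and release events set RedWorldActive and BlueWorldActive, tint the DirectionalLight, and recolor both platform types through new dynamic material instances, turning the opposite type purple.
; Tick reads both flags and enables or disables collision on every BP_RedPlatform and BP_BluePlatform, found by GetAllActorsOfClass each frame.
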(event EventTick
  (params (DeltaSeconds :type Float%20%28single-precision%29))
  (Utilities|FlowControl|Sequence
    (:then_0
      ;[1 1 1] COLLISION BLUE
      (bind _outactors (Actor|GetAllActorsOfClass "/Game/Blueprints/BP_BluePlatform.BP_BluePlatform_C"))
      (if (Variables|Default|GetblueWorldActive)
        (for _array_element _outactors
          (Collision|SetCollisionEnabled (Variables|/Script/Engine.StaticMeshActor|GetStaticMeshComponent _array_element) "QueryAndPhysics")
          (Actor|GetActorOfClass "/Game/Blueprints/GameModeClasses/BP_RunningCharacter.BP_RunningCharacter_C"))
        (else
          (for _array_element_2 _outactors
            (Collision|SetCollisionEnabled (Variables|/Script/Engine.StaticMeshActor|GetStaticMeshComponent _array_element_2) "NoCollision")))))
    (:then_1
      ;[1 1 1] COLLISION RED
      (bind _outactors_2 (Actor|GetAllActorsOfClass "/Game/Blueprints/BP_RedPlatform.BP_RedPlatform_C"))
      (if (Variables|Default|GetredWorldActive)
        (for _array_element_3 _outactors_2
          (Collision|SetCollisionEnabled (Variables|/Script/Engine.StaticMeshActor|GetStaticMeshComponent _array_element_3) "QueryAndPhysics"))
        (else
          (for _array_element_4 _outactors_2
            (Collision|SetCollisionEnabled (Variables|/Script/Engine.StaticMeshActor|GetStaticMeshComponent _array_element_4) "NoCollision")))))))

(event Input|MouseEvents|LeftMouseButton
  (params (Key :type Key%20Structure :default "None"))
  ;[1 1 1] LEFT MOUSE BUTTON
  (:Pressed
    (Development|PrintString "redON")
    (bind _returnvalue (Actor|GetActorOfClass "/Script/Engine.DirectionalLight"))
    (Rendering|Components|Light|SetLightColor (Variables|/Script/Engine.Light|GetLightComponent _returnvalue) "(R=1.000000,G=0.241667,B=0.367420,A=1.000000)" true)
    (Utilities|FlowControl|Sequence
      (:then_0
        (bind _outactors (Actor|GetAllActorsOfClass "/Game/Blueprints/BP_RedPlatform.BP_RedPlatform_C"))
        (for _array_element _outactors
          (bind _returnvalue_2 (Rendering|Material|CreateDynamicMaterialInstance (Actor|GetComponentbyClass _array_element "/Script/Engine.StaticMeshComponent") 0 0 "None" :!class /Script/Engine.PrimitiveComponent))
          (Rendering|Material|SetVectorParameterValue _returnvalue_2 "color" "(R=0.886275,G=0.105882,B=0.235294,A=1.000000)" :!class /Script/Engine.MaterialInstanceDynamic)
          (Utilities|FlowControl|Sequence
            (:then_0
              (Variables|Default|SetblueWorldActive false))
            (:then_1
              (Variables|Default|SetredWorldActive true)))))
      (:then_1
        (bind _outactors_2 (Actor|GetAllActorsOfClass "/Game/Blueprints/BP_BluePlatform.BP_BluePlatform_C"))
        (for _array_element_2 _outactors_2
          (bind _returnvalue_3 (Rendering|Material|CreateDynamicMaterialInstance (Actor|GetComponentbyClass _array_element_2 "/Script/Engine.StaticMeshComponent") 0 0 "None" :!class /Script/Engine.PrimitiveComponent))
          (Rendering|Material|SetVectorParameterValue _returnvalue_3 "color" "(R=0.517647,G=0.058824,B=1.000000,A=1.000000)" :!class /Script/Engine.MaterialInstanceDynamic)))))
  (:Released
    (Development|PrintString "redOFF")
    (bind _returnvalue_4 (Actor|GetActorOfClass "/Script/Engine.DirectionalLight"))
    (Rendering|Components|Light|SetLightColor (Variables|/Script/Engine.Light|GetLightComponent _returnvalue_4) "(R=1.000000,G=1.000000,B=1.000000,A=1.000000)" true)
    (Utilities|FlowControl|Sequence
      (:then_0
        (bind _outactors_3 (Actor|GetAllActorsOfClass "/Game/Blueprints/BP_RedPlatform.BP_RedPlatform_C"))
        (for _array_element_3 _outactors_3
          (bind _returnvalue_5 (Rendering|Material|CreateDynamicMaterialInstance (Actor|GetComponentbyClass _array_element_3 "/Script/Engine.StaticMeshComponent") 0 0 "None" :!class /Script/Engine.PrimitiveComponent))
          (Rendering|Material|SetVectorParameterValue _returnvalue_5 "color" "(R=0.886275,G=0.105882,B=0.235294,A=0.501961)" :!class /Script/Engine.MaterialInstanceDynamic)
          (Variables|Default|SetredWorldActive false)))
      (:then_1
        (bind _outactors_4 (Actor|GetAllActorsOfClass "/Game/Blueprints/BP_BluePlatform.BP_BluePlatform_C"))
        (for _array_element_4 _outactors_4
          (bind _returnvalue_6 (Rendering|Material|CreateDynamicMaterialInstance (Actor|GetComponentbyClass _array_element_4 "/Script/Engine.StaticMeshComponent") 0 0 "None" :!class /Script/Engine.PrimitiveComponent))
          (Rendering|Material|SetVectorParameterValue _returnvalue_6 "color" "(R=0.176471,G=0.235294,B=0.843137,A=0.501961)" :!class /Script/Engine.MaterialInstanceDynamic))))))

(event Input|MouseEvents|RightMouseButton
  (params (Key :type Key%20Structure :default "None"))
  ;[1 1 1] RIGHT MOUSE BUTTON
  (:Pressed
    (Development|PrintString "blueON")
    (bind _returnvalue (Actor|GetActorOfClass "/Script/Engine.DirectionalLight"))
    (Rendering|Components|Light|SetLightColor (Variables|/Script/Engine.Light|GetLightComponent _returnvalue) "(R=0.231373,G=0.270588,B=0.600000,A=1.000000)" true)
    (Utilities|FlowControl|Sequence
      (:then_0
        (bind _outactors (Actor|GetAllActorsOfClass "/Game/Blueprints/BP_BluePlatform.BP_BluePlatform_C"))
        (for _array_element _outactors
          (bind _returnvalue_2 (Rendering|Material|CreateDynamicMaterialInstance (Actor|GetComponentbyClass _array_element "/Script/Engine.StaticMeshComponent") 0 0 "None" :!class /Script/Engine.PrimitiveComponent))
          (Rendering|Material|SetVectorParameterValue _returnvalue_2 "color" "(R=0.176471,G=0.235294,B=0.843137,A=1.000000)" :!class /Script/Engine.MaterialInstanceDynamic)
          (Utilities|FlowControl|Sequence
            (:then_0
              (Variables|Default|SetblueWorldActive true))
            (:then_1
              (Variables|Default|SetredWorldActive false)))))
      (:then_1
        (bind _outactors_2 (Actor|GetAllActorsOfClass "/Game/Blueprints/BP_RedPlatform.BP_RedPlatform_C"))
        (for _array_element_2 _outactors_2
          (bind _returnvalue_3 (Rendering|Material|CreateDynamicMaterialInstance (Actor|GetComponentbyClass _array_element_2 "/Script/Engine.StaticMeshComponent") 0 0 "None" :!class /Script/Engine.PrimitiveComponent))
          (Rendering|Material|SetVectorParameterValue _returnvalue_3 "color" "(R=0.517647,G=0.058824,B=1.000000,A=1.000000)" :!class /Script/Engine.MaterialInstanceDynamic)))))
  (:Released
    (Development|PrintString "blueOFF")
    (bind _returnvalue_4 (Actor|GetActorOfClass "/Script/Engine.DirectionalLight"))
    (Rendering|Components|Light|SetLightColor (Variables|/Script/Engine.Light|GetLightComponent _returnvalue_4) "(R=1.000000,G=1.000000,B=1.000000,A=1.000000)" true)
    (Utilities|FlowControl|Sequence
      (:then_0
        (bind _outactors_3 (Actor|GetAllActorsOfClass "/Game/Blueprints/BP_BluePlatform.BP_BluePlatform_C"))
        (for _array_element_3 _outactors_3
          (bind _returnvalue_5 (Rendering|Material|CreateDynamicMaterialInstance (Actor|GetComponentbyClass _array_element_3 "/Script/Engine.StaticMeshComponent") 0 0 "None" :!class /Script/Engine.PrimitiveComponent))
          (Rendering|Material|SetVectorParameterValue _returnvalue_5 "color" "(R=0.176471,G=0.235294,B=0.843137,A=0.501961)" :!class /Script/Engine.MaterialInstanceDynamic)
          (Variables|Default|SetblueWorldActive false)))
      (:then_1
        (bind _outactors_4 (Actor|GetAllActorsOfClass "/Game/Blueprints/BP_RedPlatform.BP_RedPlatform_C"))
        (for _array_element_4 _outactors_4
          (bind _returnvalue_6 (Rendering|Material|CreateDynamicMaterialInstance (Actor|GetComponentbyClass _array_element_4 "/Script/Engine.StaticMeshComponent") 0 0 "None" :!class /Script/Engine.PrimitiveComponent))
          (Rendering|Material|SetVectorParameterValue _returnvalue_6 "color" "(R=0.886275,G=0.105882,B=0.235294,A=0.501961)" :!class /Script/Engine.MaterialInstanceDynamic))))))